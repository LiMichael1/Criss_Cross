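; The player-controlled chicken in a road-crossing game with water, logs, vehicles, trucks and trains.
; Axis inputs add movement that Tick consumes as a swept local offset, and Jump plays a cluck.
; Overlap casts choose the outcome: logs snap the chicken's Y once, traffic destroys it with a squawk, and trains add crash particles.
; Water calls an empty StopCamera, then Drown sinks it within one frame before particles, squawk and destruction.
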(event `InputAxis|move_forward`
  (params (AxisValue :type "Float (single-precision)"))
  (`self.AddMovementInput` (`self.GetActorForwardVector`) (* AxisValue (`self.Speed`))))

(event `InputAxis|move_right`
  (params (AxisValue :type "Float (single-precision)"))
  (`self.AddMovementInput` (`self.GetActorRightVector`) (* AxisValue (`self.Speed`))))

(event `self.ReceiveTick`
  (params (DeltaSeconds :type "Float (single-precision)"))
  (bind _returnvalue (`self.ConsumeMovementInputVector`))
  (`self.K2_AddActorLocalOffset` (* _returnvalue DeltaSeconds) true))

(event `Key|A`
  (params (Key :type "Key Structure")))

(event `Key|D`
  (params (Key :type "Key Structure")))

(event `InputAction|Jump`
  (params (Key :type "Key Structure"))
  (:`Pressed`
    (`self.Jump`)
    (`GameplayStatics.PlaySound2D` "/Game/Sounds/Chicken_Clucking_Sound_Effect_-_FreeSFX.Chicken_Clucking_Sound_Effect_-_FreeSFX" 1.0 1.0 0.0 null null)))

(event `self.ReceiveActorBeginOverlap`
  (params (OtherActor :type "Actor Object Reference"))
  (bind (_returnvalue_x _returnvalue_y) (`KismetMathLibrary.BreakVector` (`self.K2_GetActorLocation` (`self.Cur Log`))))
  (cast `/Game/Blueprints/bp_water` OtherActor
    (:`then`
      (`self.Stop Camera`)
      (`self.Drown`))
    (:`CastFailed`
      (bind _asbp_log (cast `/Game/Blueprints/bp_log` OtherActor)
        (:`then`
          (set `self.Cur Log` _asbp_log)
          (`self.K2_SetActorLocation` (`KismetMathLibrary.MakeVector` 0.0 _returnvalue_y)))
        (:`CastFailed`
          (cast `/Game/Blueprints/bp_vehicle` OtherActor
            (:`then`
              (`self.Hit by Vehicle`))
            (:`CastFailed`
              (cast `/Game/Blueprints/bp_truck` OtherActor
                (:`then`
                  (`self.Hit by Vehicle`))
                (:`CastFailed`
                  (cast `/Game/Blueprints/bp_train` OtherActor)
                  (`self.Hit by Train`))))))))))

(event `Stop Camera`)

(event `Hit by Train`
  (`GameplayStatics.SpawnEmitterAtLocation` "/Game/ParticleSystems/PS_CrashTrain.PS_CrashTrain" (+ (`self.K2_GetActorLocation`) (0.0 0.0 50.0)))
  (`GameplayStatics.PlaySound2D` "/Game/Sounds/Chicken_Squawk_Louder_-_SFXsource_com.Chicken_Squawk_Louder_-_SFXsource_com" 1.0 1.0 0.0 null null)
  (`self.K2_DestroyActor`))

(event `Hit by Vehicle`
  (`GameplayStatics.PlaySoundAtLocation` "/Game/Sounds/Chicken_Squawk_Louder_-_SFXsource_com.Chicken_Squawk_Louder_-_SFXsource_com" (+ (`self.K2_GetActorLocation`) (0.0 0.0 50.0)) (struct) 1.0 1.0 0.0 null null null)
  (`self.K2_DestroyActor`))

(fn `Drown`
  (returns (`Is Active` :type Boolean))
  (bind (_returnvalue_x _returnvalue_y _returnvalue_z) (`KismetMathLibrary.BreakVector` (`self.K2_GetActorLocation`)))
  (for _ (range 101)
    (`self.K2_SetActorLocation` (`KismetMathLibrary.MakeVector` 0.0 0.0 (- _returnvalue_z 1.0))))
  (`GameplayStatics.SpawnEmitterAtLocation` "/Game/ParticleSystems/PS_Drown.PS_Drown")
  (`GameplayStatics.PlaySound2D` "/Game/Sounds/Chicken_Squawk_Louder_-_SFXsource_com.Chicken_Squawk_Louder_-_SFXsource_com" 1.0 1.0 0.0 null null)
  (`self.K2_DestroyActor`)
  (return false))

(fn `UserConstructionScript`)