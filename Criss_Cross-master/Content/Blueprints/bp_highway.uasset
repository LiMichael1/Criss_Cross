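; Highway traffic spawner that periodically creates cars and trucks and removes them at kill volumes.
; A frame counter on Tick randomly calls SpawnCar or SpawnTruck roughly every 50 frames, so traffic rate follows frame rate.
; Each spawn uses the relative location of one of three type-specific spawn components and plays 2D horn and passing sounds.
; Two KillVehicle overlap components destroy entering bp_truck or bp_vehicle actors; DestroyVehicle is an empty stub.
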(event `self.ReceiveTick`
  (params (DeltaSeconds :type "Float (single-precision)"))
  (bind _result (`/Engine/EditorBlueprintResources/StandardMacros.IncrementInt` (`self.counter`))
    (:`  `
      (if (> _result 50)
        (switch `int` (`KismetMathLibrary.RandomIntegerInRange` 0 1)
          (:`0`
            (`self.SpawnCar`))
          (:`1`
            (`self.SpawnTruck`)))
        (set `self.counter` 0)))))

(event `self.ReceiveBeginPlay`)

(event `self.KillVehicle1.OnComponentBeginOverlap`
  (params (OverlappedComponent :type "PrimitiveComponent Object Reference") (OtherActor :type "Actor Object Reference") (OtherComp :type "PrimitiveComponent Object Reference") (OtherBodyIndex :type Integer) (bFromSweep :type Boolean) (SweepResult :type "HitResult Structure (by ref)"))
  (bind _asbp_truck (cast `/Game/Blueprints/bp_truck` OtherActor)
    (:`then`
      (`self.K2_DestroyActor` _asbp_truck))
    (:`CastFailed`
      (bind _asbp_vehicle (cast `/Game/Blueprints/bp_vehicle` OtherActor))
      (`self.K2_DestroyActor` _asbp_vehicle))))

(event `self.KillVehicle2.OnComponentBeginOverlap`
  (params (OverlappedComponent :type "PrimitiveComponent Object Reference") (OtherActor :type "Actor Object Reference") (OtherComp :type "PrimitiveComponent Object Reference") (OtherBodyIndex :type Integer) (bFromSweep :type Boolean) (SweepResult :type "HitResult Structure (by ref)"))
  (bind _asbp_truck (cast `/Game/Blueprints/bp_truck` OtherActor)
    (:`then`
      (`self.K2_DestroyActor` _asbp_truck))
    (:`CastFailed`
      (bind _asbp_vehicle (cast `/Game/Blueprints/bp_vehicle` OtherActor))
      (`self.K2_DestroyActor` _asbp_vehicle))))

(fn `DestroyVehicle`)

(fn `SpawnCar`
  (`|SpawnActorFromClass` "/Game/Blueprints/bp_vehicle.bp_vehicle_C" (`KismetMathLibrary.MakeTransform` (`SceneComponent.RelativeLocation` (select `int` (`KismetMathLibrary.RandomIntegerInRange` 0 2) :`0` (`self.CarSpawn1`) :`1` (`self.CarSpawn2`) :`2` (`self.CarSpawn3`)))) "Undefined" "OverrideRootScale" null null)
  (`|ExecutionSequence`
    (:`then_0`
      (`GameplayStatics.PlaySound2D` "/Game/Sounds/Car_horn_sound_effect__Copyright_Free__-_SoundEffects.Car_horn_sound_effect__Copyright_Free__-_SoundEffects" 1.0 1.0 0.0 null null))
    (:`then_1`
      (`GameplayStatics.PlaySound2D` "/Game/Sounds/car_passing_sound_-_justsoundfx.car_passing_sound_-_justsoundfx" 1.0 1.0 0.0 null null))
    (:`then_2`
      (`GameplayStatics.PlaySound2D` "/Game/Sounds/car_passing_sound_-_justsoundfx.car_passing_sound_-_justsoundfx" 1.0 1.0 0.0 null null))))

(fn `SpawnTruck`
  (`|SpawnActorFromClass` "/Game/Blueprints/bp_truck.bp_truck_C" (`KismetMathLibrary.MakeTransform` (`SceneComponent.RelativeLocation` (select `int` (`KismetMathLibrary.RandomIntegerInRange` 0 2) :`0` (`self.TruckSpawn1`) :`1` (`self.TruckSpawn2`) :`2` (`self.TruckSpawn3`)))) "Undefined" "OverrideRootScale" null null)
  (`|ExecutionSequence`
    (:`then_0`
      (`GameplayStatics.PlaySound2D` "/Game/Sounds/Car_horn_sound_effect__Copyright_Free__-_SoundEffects.Car_horn_sound_effect__Copyright_Free__-_SoundEffects" 1.0 1.0 0.0 null null))
    (:`then_1`
      (`GameplayStatics.PlaySound2D` "/Game/Sounds/car_passing_sound_-_justsoundfx.car_passing_sound_-_justsoundfx" 1.0 1.0 0.0 null null))
    (:`then_2`
      (`GameplayStatics.PlaySound2D` "/Game/Sounds/car_passing_sound_-_justsoundfx.car_passing_sound_-_justsoundfx" 1.0 1.0 0.0 null null))))

(fn `UserConstructionScript`)