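; Chicken is a player-controlled pawn that moves from the move_forward and move_right input axes.
; Each axis feeds movement input along the actor's forward or right vector, scaled by Speed.
; Tick consumes that input and applies it, scaled by delta time, as a swept local offset, although the input vectors are in world space.
; Two 90-degree yaw rotation snippets are left unconnected and never run.
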(event `InputAxis|move_forward`
  (params (AxisValue :type "Float (single-precision)"))
  (`self.AddMovementInput` (`self.GetActorForwardVector`) (* AxisValue (`self.speed`))))

(event `InputAxis|move_right`
  (params (AxisValue :type "Float (single-precision)"))
  (`self.AddMovementInput` (`self.GetActorRightVector`) (* AxisValue (`self.speed`))))

(event `self.ReceiveTick`
  (params (DeltaSeconds :type "Float (single-precision)"))
  (bind _returnvalue (`self.ConsumeMovementInputVector`))
  (`self.K2_AddActorLocalOffset` (* _returnvalue DeltaSeconds) true))

(event `Key|A`
  (params (Key :type "Key Structure")))

(event `Key|D`
  (params (Key :type "Key Structure")))

(fn `UserConstructionScript`)