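; Train track actor that periodically spawns trains and removes them at the end of the track.
; It spawns a train on BeginPlay and again whenever a per-frame Tick counter passes a fixed threshold, so timing depends on frame rate.
; Each spawn uses the Spawn component's relative location and plays crossing, horn and passing-vehicle sounds in 2D.
; Trains overlapping the DestroyTrain component are destroyed.
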(event `self.ReceiveBeginPlay`
  (`self.SpawnTrain`))

(event `self.ReceiveTick`
  (params (DeltaSeconds :type "Float (single-precision)"))
  (bind _result (`/Engine/EditorBlueprintResources/StandardMacros.IncrementInt` (`self.counter`))
    (:`  `
      (if (> _result 500)
        (`self.SpawnTrain`)
        (set `self.counter` 0)))))

(event `self.Destroy Train.OnComponentBeginOverlap`
  (params (OverlappedComponent :type "PrimitiveComponent Object Reference") (OtherActor :type "Actor Object Reference") (OtherComp :type "PrimitiveComponent Object Reference") (OtherBodyIndex :type Integer) (bFromSweep :type Boolean) (SweepResult :type "HitResult Structure (by ref)"))
  (bind _asbp_train (cast `/Game/Blueprints/bp_train` OtherActor))
  (`self.K2_DestroyActor` _asbp_train))

(fn `SpawnTrain`
  (`|SpawnActorFromClass` "/Game/Blueprints/bp_train.bp_train_C" (`KismetMathLibrary.MakeTransform` (`SceneComponent.RelativeLocation` (`self.Spawn`))) "Undefined" "OverrideRootScale" null null)
  (`|ExecutionSequence`
    (:`then_0`
      (`GameplayStatics.PlaySound2D` "/Game/Sounds/Railroad_Crossing.Railroad_Crossing" 1.0 1.0 0.0 null null))
    (:`then_1`
      (`GameplayStatics.PlaySound2D` "/Game/Sounds/Train_Horns_Sound_Effect_-_OnlineIncomeWiki.Train_Horns_Sound_Effect_-_OnlineIncomeWiki" 1.0 1.0 0.0 null null))
    (:`then_2`
      (`GameplayStatics.PlaySound2D` "/Game/Sounds/Large_Truck_Passing_On_Highway_-_Audio_Library.Large_Truck_Passing_On_Highway_-_Audio_Library" 1.0 1.0 0.0 null null))))

(fn `UserConstructionScript`)